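; Base enemy character with a camera-facing health bar, driven by an AI controller and exposing damage, healing, patrol route and movement speed functions.
; BPC_DamageSystem handles health; hits freeze the AI, play a reaction, then switch it to attacking the damage causer.
; Attacks reserve tokens from the target, tracked per target and returned on attack end or death.
; Death stops AI logic, plays sound and montage, scatters random loot, then destroys the actor.
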(event OnDeath(BPC_DamageSystem)
  ;[1 0.04992 0] Death
  (Pawn|Components|CharacterMovement|SetMovementMode (Variables|Character|GetCharacterMovement) "MOVE_None" 0)
  (Rendering|SetVisibility (Variables|Default|GetHealthBarWidget) false false)
  (AI|Logic|StopLogic (Variables|/Script/AIModule.AIController|GetBrainComponent (Variables|Default|GetAIController%20Enemy%20Base)) "")
  (bind _keys (Utilities|Map|Keys (Variables|Default|GetReservedAttackTokens)))
  (for _array_element _keys
    (Class|BPIDamagable|ReturnAttackToken(Message) _array_element (.Value (Utilities|Map|Find (Variables|Default|GetReservedAttackTokens) 0))))
  (Default|SetStateasDead (Variables|Default|GetAIController%20Enemy%20Base))
  (Utilities|FlowControl|DoOnce false
    (:Completed
      (Audio|PlaySoundatLocation (Variables|Default|GetDeathSound) (Transformation|GetActorLocation) "0, 0, 0" 0.3 1.0 0.0 0 0 0 0)
      (for _index (range 0 (Math|Random|RandomIntegerinRange 2 4))
        (CallFunction|DropLoot))
      (Animation|Montage|PlayMontage (Variables|Character|GetMesh) (Variables|Default|GetDeathMontage)
        (:OnBlendOut
          (Actor|DestroyActor))))))

(event OnDamageResponce(BPC_DamageSystem)
  (params (DamageResponse :type Enum_DamageResponses%20Enum :default "NewEnumerator0") (DamageCauser :type Actor%20Object%20Reference))
  (bind _aicontroller_enemy_base (Variables|Default|GetAIController%20Enemy%20Base))
  ;[1 1 1] On Damage Responce
  (Components|Movement|StopMovementImmediately (Variables|Character|GetCharacterMovement))
  (bind _state (Default|GetCurrentState (Variables|Default|GetAIController%20Enemy%20Base)))
  (if (Utilities|Enum|NotEqual(Enum) _state "NewEnumerator2")
    (Default|SetStateasFrozen _aicontroller_enemy_base)
    (Animation|Montage|PlayMontage (Variables|Character|GetMesh) (Variables|Default|GetHitReactionMontage)
      (:OnCompleted
        _)
      (:OnInterrupted
        _))
    (Default|SetStateasAttack _aicontroller_enemy_base DamageCauser true)))

(event Custom|DropLoot
  (bind _returnvalue (Math|Random|RandomIntegerinRange 50 150))
  ;[0.1582 0.8296 1] Spawn Random Loot
  (if (<= (Variables|Default|GetDropChance) 100)
    (Game|SpawnActorfromClass (Utilities|Select :Index (Math|Random|RandomInteger 4) :Option%200 "/Game/GameObjects/Loot/BPC_Money.BPC_Money_C" :Option%201 "/Game/GameObjects/Loot/BPC_RareMoney.BPC_RareMoney_C" :Option%202 "/Game/GameObjects/Loot/BPC_Heal.BPC_Heal_C" :Option%203 "/Game/GameObjects/Loot/BPC_Ammo.BPC_Ammo_C") (Math|Conversions|ToTransform(Vector) (+ (Transformation|GetActorLocation) (Math|Vector|MakeVector (Math|Conversions|ToFloat(Integer) _returnvalue) (Math|Conversions|ToFloat(Integer) _returnvalue) 0.0))) "Undefined" "MultiplyWithRoot" 0 0)))

(event EventBeginPlay
  ;[0 0 0] Begin Play
  (bind _returnvalue (UserInterface|CreateWidget "/Game/DamageSystem/Enemy_HealthBar.Enemy_HealthBar_C" 0 self))
  (UserInterface|SetWidget (Variables|Default|GetHealthBarWidget) _returnvalue)
  (bind _asaicontroller_enemy_base (Utilities|Casting|CastToAIController_EnemyBase (AI|GetAIController self)))
  (Variables|Default|SetAIController%20Enemy%20Base _asaicontroller_enemy_base))

(event EventTick
  (params (DeltaSeconds :type Float%20%28single-precision%29))
  ;[1 1 1] Happens every frame
  (Transformation|SetWorldRotation (Variables|Default|GetHealthBarWidget) (Math|Rotator|FindLookatRotation (Transformation|GetActorLocation) (Transformation|GetActorLocation (Game|GetPlayerCameraManager 0))) false false))

(event EventStoreAttackTokens
  (params (AttackTarget :type Actor%20Object%20Reference) (Amount :type Integer))
  (bind _reservedattacktokens (Variables|Default|GetReservedAttackTokens))
  (bind (_value _returnvalue) (Utilities|Map|Find _reservedattacktokens AttackTarget))
  ;[1 1 1] Token implementaion
  (Utilities|Map|Add (Variables|Default|GetReservedAttackTokens) AttackTarget (Math|Integer|SelectInt (+ Amount _value) Amount _returnvalue)))

(event EventAttack
  (params (AttackTarget :type Actor%20Object%20Reference))
  ;[1 1 1] Token implementaion
  (Variables|Default|SetAttacking true))

(event EventAttackEnd
  (params (AttackTarget :type Actor%20Object%20Reference))
  (bind _tokensusedincurrentattack (Variables|Default|GetTokensUsedInCurrentAttack))
  ;[1 1 1] Token implementaion
  (Class|BPIDamagable|ReturnAttackToken(Message) AttackTarget _tokensusedincurrentattack)
  (CallFunction|StoreAttackTokens AttackTarget (* _tokensusedincurrentattack -1))
  (Default|CallOnAttackEnd))

(fn ConstructionScript)

(fn AttackStart
  (params (AttackTarget :type Actor%20Object%20Reference) (TokensRequired :type Integer))
  (bind _success (Class|BPIDamagable|ReserveAttackToken(Message) AttackTarget TokensRequired))
  (if _success
    (CallFunction|StoreAttackTokens AttackTarget TokensRequired)
    (Variables|Default|SetTokensUsedInCurrentAttack TokensRequired)
    (return true)
    (else
      (return false))))

(fn GetCurrentHealth
  (return (Variables|/Game/DamageSystem/BPC_DamageSystem.BPC_DamageSystem_C|GetcurrentHealth (Variables|Default|GetBPC_DamageSystem))))

(fn GetIdealRange
  (return 1.5e+02 3.5e+02))

(fn GetMaxHealth
  (return (Variables|/Game/DamageSystem/BPC_DamageSystem.BPC_DamageSystem_C|GetmaxHealth (Variables|Default|GetBPC_DamageSystem))))

(fn GetPatrolRoute
  (return (Variables|AI|GetPatrolRoute)))

(fn Heal
  (params (Amount :type Float%20%28double-precision%29))
  (bind _newhealth (Default|Heal (Variables|Default|GetBPC_DamageSystem) Amount))
  (return _newhealth))

(fn IsAttacking
  (return (Variables|Default|GetAttacking)))

(fn IsDead
  (return (Variables|/Game/DamageSystem/BPC_DamageSystem.BPC_DamageSystem_C|GetIsDead (Variables|Default|GetBPC_DamageSystem))))

(fn ReserveAttackToken
  (params (Amount :type Integer))
  (return false))

(fn SetMovementSpeed
  (params (Speed :type Enum_MovementSpeed%20Enum :default "NewEnumerator0"))
  (bind _output_get (Variables|/Script/Engine.CharacterMovementComponent|SetMaxWalkSpeed (Variables|Character|GetCharacterMovement) (Utilities|Select :Index Speed :NewEnumerator0 0.0 :NewEnumerator1 2e+02 :NewEnumerator2 4e+02 :NewEnumerator3 6e+02)))
  (return _output_get))

(fn TakeDamage
  (params (DamageInfo :type S%20Damage%20Info%20Structure) (Damage%20Causer :type Actor%20Object%20Reference))
  (bind _wasdamaged (Default|TakeDamage (Variables|Default|GetBPC_DamageSystem) DamageInfo Damage%20Causer))
  (return _wasdamaged))