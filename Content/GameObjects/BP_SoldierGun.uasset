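; Player rifle pickup that attaches to the player's mesh socket, fills its magazine and creates the ammo UI.
; Firing spends a round, plays montage, sound and muzzle effect, emits AI noise, and line-traces from the follow camera, sending damage and spawning impacts on hits.
; Reload, enabled after a hit, moves reserve ammo into the magazine and blocks shooting during a short delay.
; Drop detaches the gun and enables gravity on its sphere.
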(event Custom|PickUp
  (params (Character :type Actor%20Object%20Reference))
  ;[1 0.8876 0.07081] Pickup Gun
  (Components|Activation|Deactivate (Variables|Default|GetRotatingMovement))
  (Transformation|AttachComponentToComponent (Variables|/Script/Engine.Character|GetMesh (Variables|Default|GetAs%20BP%20Player)) (Variables|Default|GetSocketToAttachTo) "SnapToTarget" "SnapToTarget" "KeepWorld" true)
  (Default|WeaponAssign (Variables|Default|GetAs%20BP%20Player) self)
  (CallFunction|UpdateAmmo))

(event Custom|OnPlayerDied_Event
  ;[1 1 1] BeginPlay
  (bind _asbp_player (Utilities|Casting|CastToBP_Player (Game|GetPlayerCharacter 0)))
  (Variables|Default|SetAs%20BP%20Player _asbp_player))

(event Custom|FireTrace
  (bind _self self)
  (bind _as_bp_player (Variables|Default|GetAs%20BP%20Player))
  (bind _as_bp_player_2 (Variables|Default|GetAs%20BP%20Player))
  (bind _shootsocket (Variables|Default|GetShootSocket))
  (bind _as_bp_player_3 (Variables|Default|GetAs%20BP%20Player))
  (bind _returnvalue (Transformation|GetActorLocation _self))
  (bind _followcamera (Variables|/Game/Player/BP_Player.BP_Player_C|GetFollowCamera _as_bp_player_2))
  (bind _returnvalue_2 (Transformation|GetWorldLocation _followcamera))
  ;[1 0.1691 0] Firing system
  (if (> (Variables|Default|GetAmmoInMag) 0)
    (if (Variables|Default|GetcanShoot)
      (Variables|Default|SetAmmoInMag (- (Variables|Default|GetAmmoInMag) 1))
      (Animation|Montage|PlayMontage (Variables|/Script/Engine.Character|GetMesh (Variables|Default|GetAs%20BP%20Player)) "/Game/Player/PlayerAnimation/Animation/FireRifle_Montage.FireRifle_Montage"
        (:then
          (Utilities|FlowControl|Sequence
            (:then_0
              (Audio|PlaySoundatLocation "/Game/Sound/Weapon/MS_Gun.MS_Gun" _returnvalue "0, 0, 0" 1.0 1.0 0.0 0 0 0 0)
              (Class|Actor|MakeNoise _as_bp_player 1.0 _as_bp_player _returnvalue 0.0 "None")
              (bind (_outhit _returnvalue_3) (Collision|LineTraceByChannel _returnvalue_2 (+ _returnvalue_2 (* (Math|Vector|GetForwardVector _followcamera) (Variables|Default|GetGun%20Range))) "TraceTypeQuery1" false 0 "None" true "(R=1.000000,G=0.000000,B=0.000000,A=1.000000)" "(R=0.000000,G=1.000000,B=0.000000,A=1.000000)" 2.5))
              (if _returnvalue_3
                (if (not (== (.HitActor (Collision|BreakHitResult _outhit)) _as_bp_player_3))
                  (Class|BPIDamagable|TakeDamage(Message) (.HitActor (Collision|BreakHitResult _outhit)) (Utilities|Struct|MakeS_DamageInfo (Variables|Default|GetGunDamage) "NewEnumerator2" "NewEnumerator1" false true false true) _as_bp_player_3)
                  (Effects|SpawnEmitteratLocation "/Game/Effects/Effects/FX_Monsters/FX_Monster_Troll/death/P_TrollDeathImpact.P_TrollDeathImpact" (.ImpactPoint (Collision|BreakHitResult _outhit)) (Math|Rotator|MakeRotfromX (.Normal (Collision|BreakHitResult _outhit))) "0.600000,0.600000,0.600000" true "AutoRelease")
                  (Variables|Default|SetcanBeReloaded true))))
            (:then_1
              (Effects|SpawnEmitterAttached "/Game/Effects/Effects/FX_Combat_Base/WeaponCombo/P_Combo_Finish_Ice_01.P_Combo_Finish_Ice_01" _shootsocket "None" (Transformation|GetWorldLocation _shootsocket) (Transformation|GetWorldRotation (Variables|/Game/Player/BP_Player.BP_Player_C|GetFollowCamera (Variables|Default|GetAs%20BP%20Player))) "0.150000,0.150000,0.150000" "KeepWorldPosition" true "AutoRelease"))))))
    (else
      (Audio|PlaySound2D "/Game/Sound/Weapon/Weapons_Rifle_DryFire_01.Weapons_Rifle_DryFire_01" 1.0 1.0 0.0 0 0))))

(event Custom|Drop
  (Transformation|DetachFromActor "KeepWorld" "KeepWorld" "KeepWorld")
  (Physics|SetEnableGravity (Variables|Default|GetSphere1) true))

(event Custom|Reload
  ;[0.2306 0.1735 1] Reload
  (Utilities|IsValid (Variables|/Game/Player/BP_Player.BP_Player_C|GetAs%20BP%20Soldier%20Gun (Variables|Default|GetAs%20BP%20Player))
    (:Is%20Valid
      (if (Variables|Default|GetcanBeReloaded)
        (Variables|Default|SetNeededAmmo (- (Variables|Default|GetMaxMagAmmo) (Variables|Default|GetAmmoInMag)))
        (if (and (>= (Variables|Default|GetTotalRifleAmmo) (Variables|Default|GetNeededAmmo)) (> (Variables|Default|GetNeededAmmo) 0))
          (Variables|Default|SetAmmoInMag (+ (Variables|Default|GetAmmoInMag) (Variables|Default|GetNeededAmmo)))
          (Variables|Default|SetTotalRifleAmmo (- (Variables|Default|GetTotalRifleAmmo) (Variables|Default|GetNeededAmmo)))
          (Variables|Default|SetcanShoot false :!label _label)
          (Audio|PlaySound2D "/Game/Sound/Weapon/ReloadSound.ReloadSound" 1.0 1.0 0.0 0 0)
          (Utilities|FlowControl|Delay 1.0)
          (Variables|Default|SetcanShoot true)
          (elif (and (> (Variables|Default|GetNeededAmmo) 0) (> (Variables|Default|GetTotalRifleAmmo) 0))
            (Variables|Default|SetAmmoInMag (+ (Variables|Default|GetAmmoInMag) (Variables|Default|GetTotalRifleAmmo)))
            (Variables|Default|SetTotalRifleAmmo 0)
            (goto _label)))))))

(event Custom|UpdateAmmo
  ;[0.2306 0.1735 1] Reload
  (Variables|Default|SetAmmoInMag (Variables|Default|GetMaxMagAmmo))
  (bind _returnvalue (Game|ConstructObjectfromClass "/Game/UI/Screens/AmmoUI.AmmoUI_C"))
  (UserInterface|Viewport|AddtoViewport _returnvalue 0))

(event EventBeginPlay
  ;[1 1 1] BeginPlay
  (bind _asbp_player (Utilities|Casting|CastToBP_Player (Game|GetPlayerCharacter 0)))
  (Variables|Default|SetAs%20BP%20Player _asbp_player))

(fn ConstructionScript)