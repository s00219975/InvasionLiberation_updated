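; Enemy character Blueprint that wanders randomly, chases a player it sees, and makes melee attacks until killed.
; PawnSensing triggers an AI MoveTo chase-and-attack loop that halts movement while attacking, while a three-second loop clears the seen flag and restarts wandering.
; TraceForMelee applies damage through a sphere overlap at a given bone, with hit or miss sounds.
; Damage reduces Health, shown on a camera-facing bar, and death plays a sound before destroying the actor.
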(event OnSeePawn(PawnSensing)
  (params (Pawn :type Pawn%20Object%20Reference))
  (Utilities|Casting|CastToBP_Player Pawn)
  (CallFunction|ChasePlayer Pawn)
  (Variables|Default|SethasSeenPlayer? true))

(event Custom|SearchAround
  ;[0 0.1757 1] Search Around
  (if (not (Variables|Default|GethasSeenPlayer?))
    (AI|AIMoveTo self (.RandomLocation (AI|Navigation|GetRandomReachablePointinRadius (Transformation|GetActorLocation) 2e+03 0 0)) 0 3e+02 false
      (:OnSuccess
        (Utilities|FlowControl|Delay 1.5)
        (CallFunction|SearchAround)))))

(event Custom|ChasePlayer
  (params (TargetActor :type Actor%20Object%20Reference))
  (if (not (Variables|Default|GetisDead))
    (AI|AIMoveTo self "0, 0, 0" TargetActor 1e+02 false
      (:OnSuccess
        (CallFunction|Attack)
        (Utilities|FlowControl|Delay 1.0)
        (Variables|Default|SetisAttacking false)
        (Variables|/Script/Engine.CharacterMovementComponent|SetMaxWalkSpeed (Variables|Character|GetCharacterMovement) 5e+02)
        (CallFunction|ChasePlayer TargetActor)))))

(event Custom|TraceForMelee
  (params (BoneName :type Name))
  (bind _mesh (Variables|Character|GetMesh))
  (bind _returnvalue (Transformation|GetSocketLocation _mesh BoneName))
  ;[1 1 1] Trace for Melee Attack
  (bind (_outactors _returnvalue_2) (Collision|SphereOverlapActors _returnvalue 2e+02 (Utilities|Array|MakeArray "ObjectTypeQuery3") "/Game/Player/Blueprints/BP_Player.BP_Player_C" (Utilities|Array|MakeArray self)))
  (if _returnvalue_2
    (Game|Damage|ApplyDamage (Utilities|Array|Get(acopy) _outactors) 0.1 0 0)
    (Audio|PlaySoundatLocation "/Game/Sound/Enemy/Attack/Hit.Hit" _returnvalue "0, 0, 0" 0.6 1.0 0.0 0 0 0 0)
    (else
      (Audio|PlaySoundatLocation "/Game/Sound/Enemy/Attack/MissedHit.MissedHit" _returnvalue "0, 0, 0" 1.0 1.0 0.0 0 0 0 0))))

(event Custom|Attack
  (if (not (Variables|Default|GetisDead))
    (Variables|Default|SetisAttacking true)
    (Variables|/Script/Engine.CharacterMovementComponent|SetMaxWalkSpeed (Variables|Character|GetCharacterMovement) 0.0)))

(event EventBeginPlay
  (CallFunction|SearchAround)
  (Utilities|FlowControl|Delay 3.0 :!label _label)
  (CallFunction|SearchAround)
  (Variables|Default|SethasSeenPlayer? false)
  (goto _label))

(event EventTick
  (params (DeltaSeconds :type Float%20%28single-precision%29))
  (bind _asai_health_bar_ui (Utilities|Casting|CastToAI_HealthBarUI (UserInterface|GetWidget (Variables|Default|GetHealthBarWidget))))
  (Progress|SetPercent (Variables|/Game/UI/AI_HealthBarUI.AI_HealthBarUI_C|GetProgressBar _asai_health_bar_ui) (Variables|Default|GetHealth))
  (Transformation|SetWorldRotation (Variables|Default|GetHealthBarWidget) (Math|Rotator|FindLookatRotation (Transformation|GetActorLocation) (Transformation|GetActorLocation (Game|GetPlayerCameraManager 0))) false false))

(event Game|Damage|EventAnyDamage
  (params (Damage :type Float%20%28single-precision%29) (DamageType :type Damage%20Type%20Object%20Reference) (InstigatedBy :type Controller%20Object%20Reference) (DamageCauser :type Actor%20Object%20Reference))
  ;[1 0.07796 0] Damage Taking
  (Variables|Default|SetHealth (- (Variables|Default|GetHealth) Damage))
  (if (<= (Variables|Default|GetHealth) 0.0)
    (Variables|Default|SetisDead true)
    (Pawn|Components|CharacterMovement|SetMovementMode (Variables|Character|GetCharacterMovement) "MOVE_None" 0)
    (Rendering|SetVisibility (Variables|Default|GetHealthBarWidget) false false)
    (Utilities|FlowControl|DoOnce false
      (:Completed
        (Audio|PlaySoundatLocation "/Game/Sound/Enemy/death.death" (Transformation|GetActorLocation) "0, 0, 0" 0.3 1.0 0.0 0 0 0 0)
        (Utilities|FlowControl|Delay 2.5)
        (Actor|DestroyActor)))))

(fn ConstructionScript)