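; Loot pickup that grants ammo, money or healing, chosen by its Type, when the player overlaps its sphere.
; The amount goes to the soldier gun's rifle ammo, the GameInstance currency or the player's damage system component.
; A pickup sound plays while a timeline pulls the item toward the player's attached component and shrinks it, and a short delay leads to its destruction.
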(event OnComponentBeginOverlap(SphereCollision)
  (params (OverlappedComponent :type Primitive%20Component%20Object%20Reference) (OtherActor :type Actor%20Object%20Reference) (OtherComp :type Primitive%20Component%20Object%20Reference) (OtherBodyIndex :type Integer) (bFromSweep :type Boolean) (SweepResult :type Hit%20Result%20Structure%20%28by%20ref%29))
  (bind _amounttoadd (Variables|Default|GetAmountToAdd))
  (bind _returnvalue (Math|Float|Truncate _amounttoadd))
  (if (== OtherActor (Variables|Default|GetAs%20BP%20Player))
    (switch Utilities|FlowControl|Switch|SwitchonLootTypeEnum (Variables|Default|GetType)
      (:NewEnumerator0
        ;[1 1 1] Add sound
        (CallFunction|AmmotoAdd _returnvalue))
      (:NewEnumerator1
        (CallFunction|MoneytoAdd _returnvalue))
      (:NewEnumerator2
        (CallFunction|HPtoAdd _amounttoadd)))
    (Audio|PlaySound2D "/Game/Sound/ItemPickUp.ItemPickUp" 1.0 1.0 0.0 0 0)
    (bind (_direction _locationalpha _scalealpha) (Timeline|MoneyAplha PlayFromStart)
      (:Update
        (Transformation|SetActorRelativeLocation (Math|Vector|Lerp(Vector) (Transformation|GetWorldLocation (Variables|Default|GetStaticMesh)) (Transformation|GetWorldLocation (Variables|/Game/Player/BP_Player.BP_Player_C|GetPlayerAttachedComponent (Variables|Default|GetAs%20BP%20Player))) _locationalpha))
        (Transformation|SetActorRelativeScale3D (Math|Vector|Lerp(Vector) (Transformation|GetWorldScale (Variables|Default|GetStaticMesh)) "0, 0, 0" _scalealpha))
        (Utilities|FlowControl|Delay 0.5)
        (Actor|DestroyActor)))))

(event Custom|AmmoToAdd
  (params (AmmoToPlus :type Integer))
  (bind _as_bp_player (Variables|Default|GetAs%20BP%20Player))
  (bind _as_bp_soldier_gun (Variables|/Game/Player/BP_Player.BP_Player_C|GetAs%20BP%20Soldier%20Gun _as_bp_player))
  (bind _output_get (Variables|Default|SetAmountToAdd (Math|Conversions|ToFloat(Integer) AmmoToPlus)))
  (Variables|/Game/GameObjects/BP_SoldierGun.BP_SoldierGun_C|SetTotalRifleAmmo _as_bp_soldier_gun (+ _output_get (Variables|/Game/GameObjects/BP_SoldierGun.BP_SoldierGun_C|GetTotalRifleAmmo _as_bp_soldier_gun))))

(event Custom|MoneyToAdd
  (params (CurrencyToAdd :type Integer))
  (bind _as_bp_game_instance (Variables|Default|GetAs%20BP%20Game%20Instance))
  (bind _output_get (Variables|Default|SetAmountToAdd (Math|Conversions|ToFloat(Integer) CurrencyToAdd)))
  (Variables|/Game/Player/BP_GameInstance.BP_GameInstance_C|SetCurrency _as_bp_game_instance (+ _output_get (Variables|/Game/Player/BP_GameInstance.BP_GameInstance_C|GetCurrency _as_bp_game_instance))))

(event Custom|HPToAdd
  (params (HPToAdd :type Float%20%28double-precision%29))
  (bind _output_get (Variables|Default|SetAmountToAdd HPToAdd))
  (Default|Heal (Variables|/Game/Player/BP_Player.BP_Player_C|GetBPC_DamageSystem (Variables|Default|GetAs%20BP%20Player)) _output_get))

(event EventBeginPlay
  (bind _asbp_player (Utilities|Casting|CastToBP_Player (Game|GetPlayerCharacter 0)))
  (Variables|Default|SetAs%20BP%20Player _asbp_player)
  (bind _asbp_game_instance (Utilities|Casting|CastToBP_GameInstance (Game|GetGameInstance)))
  (Variables|Default|SetAs%20BP%20Game%20Instance _asbp_game_instance))

(fn ConstructionScript)