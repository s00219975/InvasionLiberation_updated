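; BP_MeleeEnemy is a melee enemy child Blueprint that attacks with random montages, can block, and supplies its ideal attack and defend ranges.
; A montage notify fires a forward sphere trace that damages only the intended target, with hit or miss sounds.
; Blocking stops movement and flags the damage system component, whose OnBlocked event plays a reaction montage.
; A blocking state keeps that reaction from ending the block early.
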(event OnBlocked(BPC_DamageSystem)
  (params (CanBeParried :type Boolean))
  ;[0 0.5186 1] Block
  (Variables|Default|SetBlockingState "NewEnumerator2")
  (Animation|Montage|PlayMontage (Variables|Character|GetMesh) "/Game/Enemy/EnemyAnimation/EnemyBase/Animations/Block/Block_React_Montage.Block_React_Montage"
    (:OnCompleted
      _)
    (:OnInterrupted
      _))
  (CallFunction|EndBlock))

(event Custom|StartBlock
  ;[0 0.5186 1] Block
  (Components|Movement|StopMovementImmediately (Variables|Character|GetCharacterMovement))
  (Variables|/Game/DamageSystem/BPC_DamageSystem.BPC_DamageSystem_C|SetIsBlocking (Variables|Default|GetBPC_DamageSystem) true)
  (Variables|Default|SetBlockingState "NewEnumerator1")
  (Animation|Montage|PlayMontage (Variables|Character|GetMesh) "/Game/Enemy/EnemyAnimation/EnemyBase/Animations/Block/Block_Idle_Montage.Block_Idle_Montage"
    (:OnCompleted
      (CallFunction|EndBlock :!label _label))
    (:OnInterrupted
      (if (Utilities|Enum|NotEqual(Enum) (Variables|Default|GetBlockingState) "NewEnumerator2")
        (goto _label)))))

(event Custom|EndBlock
  ;[0 0.5186 1] Block
  (Variables|/Game/DamageSystem/BPC_DamageSystem.BPC_DamageSystem_C|SetIsBlocking (Variables|Default|GetBPC_DamageSystem) false)
  (Variables|Default|SetBlockingState "NewEnumerator0")
  (Default|CallOnBlockEnds))

(event EventBeginPlay
  (|CallParentFunction) ; This node is disabled and will not be called.\nDrag off pins to build functionality.
)

(event Collision|EventActorBeginOverlap
  (params (OtherActor :type Actor%20Object%20Reference)))

(event EventTick
  (params (DeltaSeconds :type Float%20%28single-precision%29))
  (|CallParentFunction DeltaSeconds) ; This node is disabled and will not be called.\nDrag off pins to build functionality.
)

(event EventAttack
  (params (AttackTarget :type Actor%20Object%20Reference))
  (bind _returnvalue (Transformation|GetActorLocation))
  (bind _returnvalue_2 (Transformation|GetActorForwardVector))
  (bind _lengthofattack (Variables|Default|GetLengthOfAttack))
  (bind _returnvalue_3 (* _returnvalue_2 _lengthofattack))
  (bind _returnvalue_4 (+ _returnvalue _returnvalue_3))
  ;[0 1 0.7751] Attack
  (|CallParentFunction AttackTarget)
  (if (not (Variables|/Game/DamageSystem/BPC_DamageSystem.BPC_DamageSystem_C|GetIsDead (Variables|Default|GetBPC_DamageSystem)))
    (bind _notifyname (Animation|Montage|PlayMontage (Variables|Character|GetMesh) (.OutItem (Utilities|Array|Random (Variables|Default|GetAttackMontage))))
      (:OnCompleted
        (CallFunction|AttackEnd AttackTarget :!label _label))
      (:OnInterrupted
        (goto _label))
      (:OnNotifyBegin
        (switch name _notifyname
          (:Slap
            (bind (_outhit _returnvalue_5) (Collision|SphereTraceForObjects _returnvalue _returnvalue_4 (Variables|Default|GetRadiusAttack) (Utilities|Array|MakeArray "ObjectTypeQuery2") false 0 "ForDuration"))
            (if _returnvalue_5
              (if (== (.HitActor (Collision|BreakHitResult _outhit)) AttackTarget)
                (Audio|PlaySoundatLocation "/Game/Sound/Enemy/Attack/Hit.Hit" _returnvalue_4 "0, 0, 0" 1.0 1.0 0.0 0 0 0 0)
                (Class|BPIDamagable|TakeDamage(Message) (.HitActor (Collision|BreakHitResult _outhit)) (Utilities|Struct|MakeS_DamageInfo (Variables|Default|GetDamage) "NewEnumerator1" "NewEnumerator1" false false false true) self)
                (else
                  (Audio|PlaySoundatLocation "/Game/Sound/Enemy/Attack/MissedHit.MissedHit" _returnvalue_4 "0, 0, 0" 1.0 1.0 0.0 0 0 0 0 :!label _label_2)))
              (else
                (goto _label_2)))))))))

(fn ConstructionScript
  (|CallParentFunction))

(fn GetIdealRange
  (return 1.5e+02 3.5e+02))