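; Ranged enemy Blueprint that spawns a gun on BeginPlay, attaches it to the right rifle socket and fires at attack targets.
; Attack plays a rifle montage, making the damage system uninterruptible until the montage completes or is interrupted, then ends the attack.
; A montage notify triggers a line trace from the gun to the target, and a hit sends blockable, force-interrupting damage to that target.
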(event Custom|EquipWeapon
  ;[0 1 0.7828] EquipWeapon
  (bind _returnvalue (Game|SpawnActorfromClass "/Game/GameObjects/BP_EnemyGun.BP_EnemyGun_C" (Math|Transform|MakeTransform "0, 0, 0") "Undefined" "MultiplyWithRoot" 0 0))
  (bind _output_get (Variables|Transformation|SetWeaponActor _returnvalue))
  (Transformation|AttachComponentToComponent _output_get (Variables|Character|GetMesh) "RightRifleSocket" "SnapToTarget" "SnapToTarget" "SnapToTarget" true))

(event EventBeginPlay
  (|CallParentFunction)
  (CallFunction|EquipWeapon))

(event Collision|EventActorBeginOverlap
  (params (OtherActor :type Actor%20Object%20Reference)))

(event EventTick
  (params (DeltaSeconds :type Float%20%28single-precision%29))
  (|CallParentFunction DeltaSeconds) ; This node is disabled and will not be called.\nDrag off pins to build functionality.
)

(event EventAttack
  (params (AttackTarget :type Actor%20Object%20Reference))
  (bind _bpc_damagesystem (Variables|Default|GetBPC_DamageSystem))
  ;[1 0.857 0] EnemyFire
  (|CallParentFunction AttackTarget)
  (bind _notifyname (Animation|Montage|PlayMontage (Variables|Character|GetMesh) "/Game/Enemy/EnemyAnimation/RangeEnemyBase/Animations/Firing_Rifle_Montage.Firing_Rifle_Montage")
    (:then
      (Variables|/Game/DamageSystem/BPC_DamageSystem.BPC_DamageSystem_C|SetIsInterruptible _bpc_damagesystem false))
    (:OnCompleted
      (CallFunction|AttackEnd AttackTarget :!label _label)
      (Variables|/Game/DamageSystem/BPC_DamageSystem.BPC_DamageSystem_C|SetIsInterruptible _bpc_damagesystem true))
    (:OnInterrupted
      (goto _label))
    (:OnNotifyBegin
      (switch name _notifyname
        (:Fire
          (bind _returnvalue (Collision|LineTraceByChannel (Transformation|GetActorLocation (Variables|Transformation|GetWeaponActor)) (Transformation|GetActorLocation AttackTarget) "TraceTypeQuery3" false 0 "None"))
          (if _returnvalue
            (Class|BPIDamagable|TakeDamage(Message) AttackTarget (Utilities|Struct|MakeS_DamageInfo (Variables|Default|GetDamage) "NewEnumerator2" "NewEnumerator1" false true false true) self)))))))

(fn ConstructionScript
  (|CallParentFunction))